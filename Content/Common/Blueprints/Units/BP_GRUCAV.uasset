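; BP_GRUCAV is a unit Blueprint whose visible logic lets the keyboard switch its action and animation state.
; Number keys 1 to 4 each pass a fixed index to SetActionByIndex, while Q and W turn animation on and off through SetAnimating.
; The construction script is empty, and neither called function is defined in this Blueprint.
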(event `Key|One` :consume false
  (params (Key :type "Key Structure" :default "AnyKey"))
  (:`Pressed`
    (`self.SetActionByIndex` 0)))

(event `Key|Two` :consume false
  (params (Key :type "Key Structure" :default "AnyKey"))
  (:`Pressed`
    (`self.SetActionByIndex` 1)))

(event `Key|Three` :consume false
  (params (Key :type "Key Structure" :default "AnyKey"))
  (:`Pressed`
    (`self.SetActionByIndex` 2)))

(event `Key|Four` :consume false
  (params (Key :type "Key Structure" :default "AnyKey"))
  (:`Pressed`
    (`self.SetActionByIndex` 3)))

(event `Key|Q` :consume false
  (params (Key :type "Key Structure" :default "AnyKey"))
  (:`Pressed`
    (`self.SetAnimating` true)))

(event `Key|W` :consume false
  (params (Key :type "Key Structure" :default "AnyKey"))
  (:`Pressed`
    (`self.SetAnimating` false)))

(fn `UserConstructionScript`)